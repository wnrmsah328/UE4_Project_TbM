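; BP_Player is a player Blueprint that implements click-to-move navigation with the mouse cursor.
; On BeginPlay it shows a crosshair cursor and enables click and mouse-over events on the player controller.
; Holding SetDestination opens a Gate on Tick, which traces under the cursor on the Visibility channel every frame.
; MoveToLocation calls SimpleMoveToLocation toward the hit point when it is at least MinClickDistance from the actor.
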(event EventBeginPlay
  (|MouseCursorSetting))

(event EventTick
  (params (DeltaSeconds :type Float%20%28single-precision%29))
  (Utilities|FlowControl|Gate true
    (:Exit
      (CallFunction|MovetoLocation (.HitResult (Game|Player|GetHitResultUnderCursorbyChannel (Game|GetPlayerController 0) "TraceTypeQuery1" true))))))

(event Input|ActionEvents|InputActionSetDestination
  (params (Key :type Key%20Structure :default "None"))
  (:Pressed
    (Utilities|FlowControl|Gate true) ; enters at Open
  )
  (:Released
    (Utilities|FlowControl|Gate true) ; enters at Close
  ))

(fn ConstructionScript)

(fn MovetoLocation
  (params (Hit :type Hit%20Result%20Structure))
  (bind _location (Collision|BreakHitResult Hit))
  (if (>= (Math|Vector|VectorLength (- _location (Transformation|GetActorLocation))) (Variables|Default|GetMinClickDistance))
    (AI|Navigation|SimpleMovetoLocation (Game|GetPlayerController 0) _location)))