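; BP_PlayerController is a player controller that implements click-and-hold movement for the controlled pawn.
; The left mouse button opens and closes a Gate, which lets Tick trace under the cursor on the Visibility channel every frame while held.
; MoveToHitLocation sends the hit point to SimpleMoveToLocation, ignoring points closer to the pawn than MinClickDistance.
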(event EventTick
  (params (DeltaSeconds :type Float%20%28single-precision%29))
  (Utilities|FlowControl|Gate true ; While key is pressed...
    (:Exit
      (CallFunction|MovetoHitLocation (.HitResult (Game|Player|GetHitResultUnderCursorbyChannel "TraceTypeQuery1" true))))))

(event Input|MouseEvents|LeftMouseButton
  (params (Key :type Key%20Structure))
  (:Pressed
    (Utilities|FlowControl|Gate true) ; enters at Open
  )
  (:Released
    (Utilities|FlowControl|Gate true) ; enters at Close
  ))

(fn ConstructionScript)

(fn MovetoHitLocation
  (params (Hit :type Hit%20Result%20Structure))
  (bind _location (Collision|BreakHitResult Hit))
  (if (>= (Math|Vector|VectorLength (- _location (Transformation|GetActorLocation (Pawn|GetControlledPawn)))) (Variables|Default|GetMinClickDistance)) ; Don't move if player clicks too close to pawn
    (AI|Navigation|SimpleMovetoLocation self _location)))